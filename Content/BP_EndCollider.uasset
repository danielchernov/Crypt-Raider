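; End-goal actor that shows the win screen when its trigger activates its Mover component.
; On BeginPlay it hands the Mover to the Trigger component, then polls the Mover's ShouldMove flag every Tick as the win signal.
; When the flag is set, it creates and displays WB_WinScreen, switches input to game and UI with a visible cursor, and pauses the game.
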(event `self.ReceiveBeginPlay`
  (`TriggerComponent.SetMover` (`self.Trigger`) (`self.Mover`)))

(event `self.ReceiveTick`
  (params (DeltaSeconds :type "Float (single-precision)"))
  (bind _returnvalue (`GameplayStatics.GetPlayerController` 0))
  (if (`Mover.ShouldMove` (`self.Mover`))
    (bind _returnvalue_2 (`|GenericCreateObject` _returnvalue "/Game/Blueprints/WB_WinScreen.WB_WinScreen_C"))
    (bind _output_get (set `self.WBWinScreen` _returnvalue_2))
    (`UserWidget.AddToViewport` _output_get 0)
    (`WidgetBlueprintLibrary.SetInputMode_GameAndUIEx` _returnvalue null)
    (set `PlayerController.bShowMouseCursor` true (`GameplayStatics.GetPlayerController` 0))
    (`GameplayStatics.SetGamePaused` true)))

(fn `UserConstructionScript`)